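; BP_Doorway_Base is a sliding doorway with an optional sensor that responds to the first-person character and Squimbus unless locked.
; DoorEntry begin and end overlaps share one toggle, playing or reversing the DoorToggle timeline to slide Door and DoorRot along Y.
; The construction script offsets both panels for doors starting open and sets FirstClose, which skips begin overlaps until an end overlap closes the door from the timeline's end.
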(event OnComponentBeginOverlap(DoorEntry)
  (params (OverlappedComponent :type Primitive%20Component%20Object%20Reference) (OtherActor :type Actor%20Object%20Reference) (OtherComp :type Primitive%20Component%20Object%20Reference) (OtherBodyIndex :type Integer) (bFromSweep :type Boolean) (SweepResult :type Hit%20Result%20Structure%20%28by%20ref%29))
  (if (Variables|Default|GetShouldOpenOnSensor)
    (if (not (Variables|StateVars|GetIsLocked))
      (if (not (Variables|StateVars|GetFirstClose))
        (Utilities|Casting|CastToBP_FirstPersonCharacter OtherActor
          (:then
            _)
          (:CastFailed
            (Utilities|Casting|CastToBP_Squimbus OtherActor)))
        (if (Variables|StateVars|GetIsOpen)
          (Variables|StateVars|SetIsMoving true)
          (Variables|StateVars|SetIsOpen false)
          (if (Variables|StateVars|GetFirstClose)
            (Variables|StateVars|SetFirstClose false)
            (bind _newtrack_0 (Timeline|DoorToggle ReverseFromEnd)
              (:Update
                (Transformation|SetRelativeLocation (Variables|Default|GetDoor) (Math|Vector|MakeVector 0.0 _newtrack_0 0.0) false true)
                (bind _result (Math|Float|NegateFloat _newtrack_0)
                  (:%20%20
                    (Transformation|SetRelativeLocation (Variables|Default|GetDoorRot) (Math|Vector|MakeVector 0.0 _result 0.0) false true))))
              (:Finished
                (Variables|StateVars|SetIsMoving false)))
            (else
              (Timeline|DoorToggle Reverse)))
          (else
            (Variables|StateVars|SetIsMoving false)
            (Variables|StateVars|SetIsOpen true)
            (Timeline|DoorToggle Play)))))))

(event OnComponentEndOverlap(DoorEntry)
  (params (OverlappedComponent :type Primitive%20Component%20Object%20Reference) (OtherActor :type Actor%20Object%20Reference) (OtherComp :type Primitive%20Component%20Object%20Reference) (OtherBodyIndex :type Integer))
  (if (Variables|Default|GetShouldOpenOnSensor)
    (if (not (Variables|StateVars|GetIsLocked))
      (Utilities|Casting|CastToBP_FirstPersonCharacter OtherActor
        (:then
          _)
        (:CastFailed
          (Utilities|Casting|CastToBP_Squimbus OtherActor)))
      (if (Variables|StateVars|GetIsOpen)
        (Variables|StateVars|SetIsMoving true)
        (Variables|StateVars|SetIsOpen false)
        (if (Variables|StateVars|GetFirstClose)
          (Variables|StateVars|SetFirstClose false)
          (bind _newtrack_0 (Timeline|DoorToggle ReverseFromEnd)
            (:Update
              (Transformation|SetRelativeLocation (Variables|Default|GetDoor) (Math|Vector|MakeVector 0.0 _newtrack_0 0.0) false true)
              (bind _result (Math|Float|NegateFloat _newtrack_0)
                (:%20%20
                  (Transformation|SetRelativeLocation (Variables|Default|GetDoorRot) (Math|Vector|MakeVector 0.0 _result 0.0) false true))))
            (:Finished
              (Variables|StateVars|SetIsMoving false)))
          (else
            (Timeline|DoorToggle Reverse)))
        (else
          (Variables|StateVars|SetIsMoving false)
          (Variables|StateVars|SetIsOpen true)
          (Timeline|DoorToggle Play))))))

(event EventBeginPlay)

(event Collision|EventActorBeginOverlap
  (params (OtherActor :type Actor%20Object%20Reference)))

(event EventTick
  (params (DeltaSeconds :type Float%20%28single-precision%29))
  (if (Variables|StateVars|GetIsMoving)
    _))

(fn ConstructionScript
  (bind _doorextents (Variables|Default|GetDoorExtents))
  (bind _returnvalue (Math|Vector|MakeVector 0.0 _doorextents 0.0))
  (if (Variables|StateVars|GetIsOpen)
    (Transformation|AddLocalOffset (Variables|Default|GetDoor) _returnvalue false true)
    (Transformation|AddLocalOffset (Variables|Default|GetDoorRot) _returnvalue false true)
    (Variables|StateVars|SetFirstClose true)))