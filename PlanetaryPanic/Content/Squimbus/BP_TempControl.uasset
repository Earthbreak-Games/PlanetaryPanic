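; Temperature control actor that slows the first-person player while it is unstable.
; Each Tick it checks IsStable, which is not defined in this Blueprint, and either calls UnstableTick or restores normal speed through ResetMaxWalkSpeed.
; Both functions cast player pawn 0 to BP_FirstPersonCharacter and write a hardcoded MaxWalkSpeed on its movement component, overwriting any other speed change every frame.
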(event EventBeginPlay
  (|CallParentFunction) ; This node is disabled and will not be called.\nDrag off pins to build functionality.
)

(event Collision|EventActorBeginOverlap
  (params (OtherActor :type Actor%20Object%20Reference))
  (|CallParentFunction OtherActor) ; This node is disabled and will not be called.\nDrag off pins to build functionality.
)

(event EventTick
  (params (DeltaSeconds :type Float%20%28single-precision%29))
  (bind _returnvalue (CallFunction|IsStable))
  (if _returnvalue
    (Utilities|ResetMaxWalkSpeed)
    (else
      (CallFunction|UnstableTick))))

(fn ConstructionScript
  (|CallParentFunction))

(fn UnstableTick
  (bind _asbp_first_person_character (Utilities|Casting|CastToBP_FirstPersonCharacter (Game|Player|GetPlayerPawn 0)))
  (Variables|/Script/Engine.CharacterMovementComponent|SetMaxWalkSpeed (Variables|/Script/Engine.Character|GetCharacterMovement _asbp_first_person_character) 4e+02))