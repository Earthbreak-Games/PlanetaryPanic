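; Repairable ship-or-world system actor whose integrity decays over time and is restored while the player interacts with it.
; OnInteract starts repair, which Tick continues until the player leaves the horizontal interaction radius, ignoring height; otherwise integrity decays.
; Both rates scale by delta time, with integrity clamped between zero and one.
; A text render shows the current integrity and turns to face the player each frame.
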(event EventBeginPlay)

(event Collision|EventActorBeginOverlap
  (params (OtherActor :type Actor%20Object%20Reference)))

(event EventTick
  (params (DeltaSeconds :type Float%20%28single-precision%29))
  (bind _isinteracting (Utilities|CheckInteractionStatus)
    (:Success
      (if _isinteracting
        (Utilities|TickRepair)
        (else
          (Utilities|TickDecay)))
      (Utilities|UpdateText))))

(fn ConstructionScript)

(fn OnInteract
  (Variables|Default|SetIsInteracting true)
  (Utilities|TickRepair))