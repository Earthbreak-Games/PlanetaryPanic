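; BP_Squimbus is an enemy character that attacks the first-person player when they enter its AttackHitbox.
; Overlap starts a one-shot TimeToAttack timer, which fires AttackPlayer to play a sound and call AttackHit on the player.
; End overlap is empty, so leaving the hitbox does not cancel a pending attack.
; Doorway overlaps only print debug text, and UpdateWalkSpeed sets movement speed.
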(event OnComponentBeginOverlap(AttackHitbox)
  (params (OverlappedComponent :type Primitive%20Component%20Object%20Reference) (OtherActor :type Actor%20Object%20Reference) (OtherComp :type Primitive%20Component%20Object%20Reference) (OtherBodyIndex :type Integer) (bFromSweep :type Boolean) (SweepResult :type Hit%20Result%20Structure%20%28by%20ref%29))
  (Utilities|Casting|CastToBP_FirstPersonCharacter OtherActor
    (:then
      (if (> (Variables|Default|GetTimeToAttack) 0.0)
        (Variables|Default|SetPlayerInRange true)
        (bind _returnvalue (Utilities|Time|SetTimerbyEvent (delegate Custom|AttackPlayer) (Variables|Default|GetTimeToAttack)))
        (Variables|Default|SetAttackTimer _returnvalue)))
    (:CastFailed
      (Utilities|Casting|CastToBP_Doorway_Base OtherActor)
      (Development|PrintText "I see you"))))

(event OnComponentEndOverlap(AttackHitbox)
  (params (OverlappedComponent :type Primitive%20Component%20Object%20Reference) (OtherActor :type Actor%20Object%20Reference) (OtherComp :type Primitive%20Component%20Object%20Reference) (OtherBodyIndex :type Integer)))

(event Custom|AttackPlayer
  (Utilities|Time|ClearandInvalidateTimerbyHandle (Variables|Default|GetAttackTimer))
  (Audio|PlaySound2D "/Game/Squimbus/SquimbSound/SC_SquimbAttack.SC_SquimbAttack" 1.0 1.0 0.0 0 0)
  (Development|PrintText "Squimb done did got you")
  (bind _asbp_first_person_character (Utilities|Casting|CastToBP_FirstPersonCharacter (Game|GetPlayerCharacter 0)))
  (Default|AttackHit _asbp_first_person_character))

(fn ConstructionScript)

(fn UpdateWalkSpeed
  (params (NewWalkSpeed :type Float%20%28double-precision%29))
  (Variables|/Script/Engine.CharacterMovementComponent|SetMaxWalkSpeed (Variables|Character|GetCharacterMovement) NewWalkSpeed))