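; BP_BackupPower is a backup power actor that clears the event manager's frozen state while it is stable.
; It inherits its BeginPlay, overlap and construction behavior from its parent class, adding logic only in Tick.
; Each tick it checks IsStable and, when true, looks up BP_EventManager with GetActorOfClass and sets FrozenState to false.
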(event EventBeginPlay
  (|CallParentFunction))

(event Collision|EventActorBeginOverlap
  (params (OtherActor :type Actor%20Object%20Reference))
  (|CallParentFunction OtherActor))

(event EventTick
  (params (DeltaSeconds :type Float%20%28single-precision%29))
  (|CallParentFunction DeltaSeconds)
  (bind _returnvalue (CallFunction|IsStable))
  (if _returnvalue
    (bind _returnvalue_2 (Actor|GetActorOfClass "/Game/Squimbus/BP_EventManager.BP_EventManager_C"))
    (Variables|/Game/Squimbus/BP_EventManager.BP_EventManager_C|SetFrozenState _returnvalue_2 false)))

(fn ConstructionScript
  (|CallParentFunction))