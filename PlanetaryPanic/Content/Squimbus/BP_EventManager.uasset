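; Event manager that drives a progress-to-win loop around repairable systems and handles win/lose endings that return to the main menu.
; Tick advances Progress while all three engines stay above their integrity thresholds and FrozenState is off.
; Progress milestones in FailureEventMap zero the mapped system's integrity, with a BackPow failure also freezing progress.
; LoseTriggered has no caller here, and the integrity-randomizing setup is disconnected.
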(event Custom|WinTriggered
  (Utilities|Time|SetTimerbyEvent (delegate Custom|LoadMainMenu) 2.0)
  (Development|PrintText "You Win!!!!!!!" true true "(R=0.022470,G=1.000000,B=0.000000,A=1.000000)")
  (Input|SetInputModeUIOnly (Game|GetPlayerController 0) 0 "DoNotLock" true))

(event Custom|LoseTriggered
  (Utilities|Time|SetTimerbyEvent (delegate Custom|LoadMainMenu) 2.0)
  (Development|PrintText "You Lose!!!!!!" true true "(R=0.022470,G=1.000000,B=0.000000,A=1.000000)")
  (Input|SetInputModeUIOnly (Game|GetPlayerController 0) 0 "DoNotLock" true))

(event Custom|LoadMainMenu
  (Game|SetGamePaused false)
  (Game|OpenLevel(byName) "MainMenu"))

(event EventBeginPlay)

(event Collision|EventActorBeginOverlap
  (params (OtherActor :type Actor%20Object%20Reference)))

(event EventTick
  (params (DeltaSeconds :type Float%20%28single-precision%29))
  (bind _values (Utilities|Map|Values (Variables|Default|GetRepairableSystems)))
  (bind _shouldprogress (CallFunction|ShouldProgress _values))
  (bind _output_get (Variables|Default|SetIsProgressing _shouldprogress))
  (if _output_get
    ;[1 1 1] doesnt update progress in event of frozen state
    (if (not (Variables|Default|GetFrozenState))
      (bind _output_get_2 (Variables|Default|SetProgress (+ (Variables|Default|GetProgress) (* DeltaSeconds (Variables|Default|GetProgressRate)))))
      (if (>= _output_get_2 1.0)
        (CallFunction|WinTriggered)
        (else
          (Utilities|FailureEventCheck))))))

(fn ConstructionScript)

(fn ShouldProgress
  (params (Array :type Array%20of%20BP%20Repairable%20System%20Object%20References))
  (LocalVariables|SetResult true)
  (bind _array_element (Utilities|Array|ForEachLoopwithBreak Array :!label _label)
    (:LoopBody
      (switch Utilities|FlowControl|Switch|SwitchonESystemType (Variables|/Game/Squimbus/BP_RepairableSystem.BP_RepairableSystem_C|GetSystemType _array_element)
        (:ST_LEngine
          (if (not (> (Variables|/Game/Squimbus/BP_RepairableSystem.BP_RepairableSystem_C|GetIntegrityPercentage _array_element) 0.25)) :!label _label_2
            (LocalVariables|SetResult false :!label _label_3)
            (goto _label Break)))
        (:ST_REngine
          (goto _label_2))
        (:ST_CEngine
          (if (not (> (Variables|/Game/Squimbus/BP_RepairableSystem.BP_RepairableSystem_C|GetIntegrityPercentage _array_element) 0.5))
            (goto _label_3)))))
    (:Completed
      (return (LocalVariables|GetResult)))))

(fn CheckforFailureEvent
  (bind _failureeventmap (Variables|Default|GetFailureEventMap))
  (bind _keys (Utilities|Map|Keys _failureeventmap))
  (bind _array_element (Utilities|Array|ForEachLoopwithBreak _keys)
    (:LoopBody
      (if (and (<= _array_element (Variables|Default|GetProgress)) (Utilities|Enum|NotEqual(Enum) (.Value (Utilities|Map|Find _failureeventmap _array_element)) (Variables|Default|GetLatestFailureEvent)))
        (if (.ReturnValue (Utilities|Map|Find (Variables|Default|GetRepairableSystems) (.Value (Utilities|Map|Find _failureeventmap _array_element))))
          (Variables|/Game/Squimbus/BP_RepairableSystem.BP_RepairableSystem_C|SetIntegrityPercentage (.Value (Utilities|Map|Find (Variables|Default|GetRepairableSystems) (.Value (Utilities|Map|Find _failureeventmap _array_element)))) 0.0)
          (bind _output_get (Variables|Default|SetLatestFailureEvent (.Value (Utilities|Map|Find _failureeventmap _array_element))))
          (if (Utilities|Enum|Equal(Enum) _output_get "ST_BackPow")
            (Variables|Default|SetFrozenState true)))))))